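; Index calculation Blueprint that picks a slot index for window wall placement in a row-based layout.
; CalculateSingle alternates by the incoming index's parity: even maps to index zero, odd to one past the total count minus a full row.
; The candidate then goes through AdjustIndexIfPossible, along with that reduced count and the occupied indices, before being returned.
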(fn `CalculateSingle`
  (params (Args :type "MBSIndexCalculationArgs Structure (by ref)"))
  (returns (ReturnValue :type Integer))
  (locals (OutIndex :type Integer))
  (bind (_buildsystem _index _initializer _occupiedindices) (`self.BreakIndexCalculationArgs` Args))
  (bind (_staticmesh _meshlist _meshlistindex _resolution _totalcount _maxinrow) (break `ModularSectionInitializer` _initializer))
  (bind _returnvalue (- _totalcount _maxinrow))
  (if (== (mod _index 2) 0)
    (set `local.OutIndex` 0)
    (else
      (set `local.OutIndex` (+ _returnvalue 1))))
  (`self.AdjustIndexIfPossible` (`local.OutIndex`) _returnvalue _occupiedindices)
  (return (`local.OutIndex`)))