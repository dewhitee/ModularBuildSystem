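; Transform solver that computes where tunnel entrance rooftop pieces go in a section-based layout.
; GetNextTransform offsets location by the default section size, using the current row for Y and the level Z multiplier for height.
; Front-facing pieces stay at zero X offset and get a half-turn yaw; back-facing ones shift by the row's maximum count in X and one more section in Y.
; Other facings are skipped.
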(fn `GetNextTransform`
  (params (Args :type "NextTransformArgs Structure (by ref)"))
  (returns (ReturnValue :type "Transform Structure"))
  (bind _returnvalue (`self.GetDefaultSectionSize`))
  (bind _returnvalue_2 (* _returnvalue (`self.GetLevelZMultiplier`)))
  (bind _returnvalue_3 (+ _returnvalue (* _returnvalue (`self.GetCurrentRow`))))
  (`self.In` Args)
  (if (`self.IsFacingFront`)
    (`self.AddLocation` (`KismetMathLibrary.MakeVector` 0.0 _returnvalue_3 _returnvalue_2))
    (`self.AddRotationYaw` -180.0)
    (elif (`self.IsFacingBack`)
      (`self.AddLocation` (`KismetMathLibrary.MakeVector` (* _returnvalue (`self.GetMaxInRow`)) (+ _returnvalue_3 _returnvalue) _returnvalue_2))
      (else
        (`self.Skip`))))
  (bind _returnvalue_4 (`self.Out`))
  (return _returnvalue_4))