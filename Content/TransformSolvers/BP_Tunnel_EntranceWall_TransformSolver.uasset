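; Transform solver that places entrance wall sections for a tunnel, overriding GetNextTransform in a grid-indexed layout.
; Only four key indices get a wall: first, end of first row, start of second row and last; all others are skipped.
; The first and last shift along X, the middle two mirror by X, and the first-row end also shifts along Y.
; Every placed wall is raised in Z by section size times level multiplier.
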(fn `GetNextTransform`
  (params (Args :type "NextTransformArgs Structure (by ref)"))
  (returns (ReturnValue :type "Transform Structure"))
  (bind _returnvalue (`self.GetDefaultSectionSize`))
  (bind _returnvalue_2 (`self.GetMaxInRow`))
  (bind _returnvalue_3 (* _returnvalue (`self.GetMaxInRow`)))
  (bind _array (`|MakeArray` 0 _returnvalue_2 (- _returnvalue_2 1) (- (`self.GetMaxCount`) 1)))
  (bind _output (`|GetArrayItem` _array 2))
  (`self.In` Args)
  (if (`self.IsIndexEqualsAnyOf` _array)
    (if (`self.IsIndexEquals` (`|GetArrayItem` _array))
      (`self.AddLocationX` (- _returnvalue_3 _returnvalue))
      (`self.AddLocationZ` (* (`self.GetDefaultSectionSize`) (`self.GetLevelZMultiplier`)) :!label _label)
      (elif (`self.IsIndexEqualsAnyOf` (`|MakeArray` (`|GetArrayItem` _array 1) _output))
        (`self.MirrorByX`)
        (if (`self.IsIndexEquals` _output)
          (`self.AddLocationY` (* (`self.GetDefaultSectionSize`) (`self.GetMaxRow`)))
          (goto _label)
          (else
            (goto _label)))
        (elif (`self.IsIndexEquals` (`|GetArrayItem` _array 3))
          (`self.AddLocationX` (+ _returnvalue_3 _returnvalue))
          (goto _label)
          (else
            (`self.Skip` :!label _label_2)))))
    (else
      (goto _label_2)))
  (bind _returnvalue_4 (`self.Out`))
  (return _returnvalue_4))