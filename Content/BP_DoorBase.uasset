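; Base door actor that swings open and closed around a rotation pivot, playing a sound at the start of each motion.
; Toggle picks Open or Close from IsOpen and ignores calls while the door is moving.
; Looping timers, rather than a Timeline despite the TimelineIsActive flag, ease the pivot's yaw with FInterpTo until near its target.
; InvertOpening flips the open angle on BeginPlay.
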(event `self.ReceiveBeginPlay`
  (if (`self.InvertOpening`)
    (set `self.OpenAngle` (* (`self.OpenAngle`) -1.0))))

(event `Toggle`
  (if (not (`self.TimelineIsActive`))
    (set `self.TimelineIsActive` true)
    (if (`self.IsOpen`)
      (`self.Close`)
      (else
        (`self.Open`)))))

(event `Open`
  (bind _returnvalue (`KismetSystemLibrary.K2_SetTimerDelegate` (delegate `OpenTick`) 0.01 true))
  (set `self.OpenCloseTimerHandle` _returnvalue)
  (`GameplayStatics.PlaySoundAtLocation` (`self.OpenSound`) (`self.K2_GetActorLocation`) (struct) 1.0 1.0 0.0 null null null null)
  (set `self.TimelineIsActive` true))

(event `OpenTick`
  (bind (_relativerotation_roll _relativerotation_pitch _relativerotation_yaw) (`KismetMathLibrary.BreakRotator` (`SceneComponent.RelativeRotation` (`self.RotationPivot`))))
  (bind _returnvalue (`KismetMathLibrary.FInterpTo` _relativerotation_yaw (`self.OpenAngle`) (`GameplayStatics.GetWorldDeltaSeconds`) (`self.InterpSpeed`)))
  (`SceneComponent.K2_SetRelativeRotation` (`self.RotationPivot`) (`KismetMathLibrary.MakeRotator` 0.0 0.0 _returnvalue) false false)
  (if (`KismetMathLibrary.NearlyEqual_FloatFloat` _returnvalue (`self.OpenAngle`) 0.1)
    (`KismetSystemLibrary.K2_ClearAndInvalidateTimerHandle` (`self.OpenCloseTimerHandle`))
    (set `self.IsOpen` true)
    (set `self.TimelineIsActive` false)))

(event `Close`
  (bind _returnvalue (`KismetSystemLibrary.K2_SetTimerDelegate` (delegate `CloseTick`) 0.01 true))
  (set `self.OpenCloseTimerHandle` _returnvalue)
  (`GameplayStatics.PlaySoundAtLocation` (`self.CloseSound`) (`self.K2_GetActorLocation`) (struct) 1.0 1.0 0.0 null null null null)
  (set `self.TimelineIsActive` true))

(event `CloseTick`
  (bind (_relativerotation_roll _relativerotation_pitch _relativerotation_yaw) (`KismetMathLibrary.BreakRotator` (`SceneComponent.RelativeRotation` (`self.RotationPivot`))))
  (bind _returnvalue (`KismetMathLibrary.FInterpTo` _relativerotation_yaw 0.0 (`GameplayStatics.GetWorldDeltaSeconds`) (`self.InterpSpeed`)))
  (`SceneComponent.K2_SetRelativeRotation` (`self.RotationPivot`) (`KismetMathLibrary.MakeRotator` 0.0 0.0 _returnvalue) false false)
  (if (`KismetMathLibrary.NearlyEqual_FloatFloat` _returnvalue 0.0 0.1)
    (`KismetSystemLibrary.K2_ClearAndInvalidateTimerHandle` (`self.OpenCloseTimerHandle`))
    (set `self.IsOpen` false)
    (set `self.TimelineIsActive` false)))

(fn `UserConstructionScript`)